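; BP_Lever is a hold-to-pull interactable lever that sends an activate message to a linked actor once it reaches its end transform.
; Interaction start and stop drive a MoveComponentTo and looping or one-shot audio, with release either halting the lever or returning it if MoveBack is set.
; Tick tracks TimeLeft so resumed pulls keep proportional duration, and reports tagged noise while moving; the cooldown timer is set past its threshold rather than accumulated, so reports repeat nearly every frame.
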(event Custom|ReportNoise
  ;[1 1 1] Reporting Noise
  (if (>= (Variables|NoiseReporting|GetNoiseReportCoolDownTimer) (Variables|NoiseReporting|GetNoiseReportCoolDown))
    (Class|AISenseHearing|ReportNoiseEvent (Transformation|GetActorLocation) 1.0 self 0.0 (Utilities|Name|EnumtoName (Variables|NoiseReporting|GetNoiseType)))))

(event EventStopInteracting
  (bind _endtransform (Variables|Default|GetEndTransform))
  (bind _lever (Variables|Default|GetLever))
  (bind _endtransform_2 (Variables|Default|GetEndTransform))
  (bind _returnvalue (Transformation|GetRelativeTransform _lever))
  ;[1 1 1] Interaction Handling
  (if (not (Variables|Moving|GetCompleted))
    (Variables|Moving|SetMoving false)
    (Audio|Components|Audio|Stop (Variables|Default|GetAudio))
    (if (Variables|Moving|GetMoveBack)
      ;[1 1 1] Moving of lever
      (Components|MoveComponentTo (Variables|Default|GetLever) (.location _endtransform) (.rotation _endtransform) false false (Variables|Moving|GetTimeLeft) false) ; enters at Return
      (else
        (Components|MoveComponentTo (Variables|Default|GetLever) (.location _endtransform) (.rotation _endtransform) false false (Variables|Moving|GetTimeLeft) false) ; enters at Stop
      ))))

(event EventTick
  (params (DeltaSeconds :type Float%20%28single-precision%29))
  ;[1 1 1] Internal timer for time left to move
  (if (Variables|Moving|GetMoving)
    (CallFunction|ReportNoise)
    (Variables|Moving|SetTimeLeft (Math|Float|Clamp(Float) (- (Variables|Moving|GetTimeLeft) DeltaSeconds) 0.0 (Variables|Moving|GetTimeToComplete)))
    (Variables|NoiseReporting|SetNoiseReportCoolDownTimer (+ (Variables|NoiseReporting|GetNoiseReportCoolDown) (Utilities|Time|GetWorldDeltaSeconds)))
    (else
      (Variables|NoiseReporting|SetNoiseReportCoolDownTimer 0.0)
      (if (Variables|Moving|GetMoveBack)
        (Variables|Moving|SetTimeLeft (Math|Float|Clamp(Float) (+ (Utilities|Time|GetWorldDeltaSeconds) (Variables|Moving|GetTimeLeft)) 0.0 (Variables|Moving|GetTimeToComplete)))))))

(event EventStartInteracting
  (params (Speed :type Float%20%28single-precision%29))
  (bind _endtransform (Variables|Default|GetEndTransform))
  (bind _lever (Variables|Default|GetLever))
  (bind _endtransform_2 (Variables|Default|GetEndTransform))
  (bind _returnvalue (Transformation|GetRelativeTransform _lever))
  ;[1 1 1] Interaction Handling
  (if (not (Variables|Moving|GetCompleted))
    (Variables|Moving|SetMoving true)
    (Audio|Components|Audio|Play (Variables|Default|GetAudio) 0.0)
    ;[1 1 1] Moving of lever
    (Components|MoveComponentTo (Variables|Default|GetLever) (.location _endtransform) (.rotation _endtransform) false false (Variables|Moving|GetTimeLeft) false)
    (bind _output_get (Variables|Moving|SetCompleted (== (Math|Transform|MakeTransform (.location _endtransform_2) (.rotation _endtransform_2) "1,1,1") (Math|Transform|MakeTransform (.location _returnvalue) (.rotation _returnvalue) "1,1,1"))))
    (if _output_get
      (Class|BPInteractable|Activate(Message) (Variables|Default|GetActorToActivate))
      (Variables|NoiseReporting|SetNoiseReportCoolDownTimer 0.0))))

(fn ConstructionScript
  (Variables|Moving|SetTimeLeft (Variables|Moving|GetTimeToComplete))
  (Transformation|SetRelativeTransform (Variables|Default|GetLever) (Variables|Default|GetStartTransform) false true))