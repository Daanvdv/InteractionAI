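; Interactive door that toggles between start and end transforms, moving faster or slower depending on the speed of the interaction.
; StartInteracting compares Speed to a threshold to pick a fast or slow duration, then sets the OpenDoor timeline's play rate from it.
; The timeline lerps the door's relative transform and tracks direction, so interacting mid-motion reverses from the current position.
; The construction script places the door at its start transform.
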(event EventStartInteracting
  (params (Speed :type Float%20%28single-precision%29))
  ;[1 1 1] Check speed of opening
  (if (> Speed (Variables|Default|GetInteractionSpeedThreshold))
    (Variables|Opening|SetTimeToOpen (Variables|Opening|GetTImeToOpenFast))
    (else
      (Variables|Opening|SetTimeToOpen (Variables|Opening|GetTImeToOpenSlow))))
  (Components|Timeline|SetPlayRate (Variables|Default|GetOpenDoor) (/ 1.0 (Variables|Opening|GetTimeToOpen)))
  (if (not (Variables|Default|GetMoving))
    (switch Utilities|FlowControl|Switch|SwitchonETimelineDirection (Variables|Default|GetTimelineDirection)
      (:Forward
        ;[1 1 1] Opening door
        (bind (_direction _completion) (Timeline|OpenDoor ReverseFromEnd)
          (:Update
            (Transformation|SetRelativeTransform (Variables|Default|GetDoor) (Math|Transform|Lerp(Transform) (Variables|Default|GetStartTransform) (Variables|Default|GetEndTransform) _completion) false false)
            (Variables|Default|SetMoving true)
            (Variables|Default|SetTimelineDirection _direction))
          (:Finished
            (Variables|Default|SetMoving false))))
      (:Backward
        (Timeline|OpenDoor PlayFromStart)))
    (else
      (switch Utilities|FlowControl|Switch|SwitchonETimelineDirection (Variables|Default|GetTimelineDirection)
        (:Forward
          (Timeline|OpenDoor Reverse))
        (:Backward
          (Timeline|OpenDoor Play))))))

(fn ConstructionScript
  (Variables|Opening|SetTimeToOpen (Variables|Opening|GetTImeToOpenSlow))
  (Transformation|SetRelativeTransform (Variables|Default|GetDoor) (Variables|Default|GetStartTransform) false true))