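; AI controller for enemies that runs BT_EnemyBehaviorTree on BeginPlay and feeds it perception results through the Blackboard.
; On a perception update, a successful sight stimulus stores the sensed actor as TargetActor and sets PlayerInVision, while lost sight only clears that flag.
; Any non-sight stimulus writes its location to TargetLocation.
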(event OnTargetPerceptionUpdated(AIPerception)
  (params (Actor :type Actor%20Object%20Reference) (Stimulus :type AI%20Stimulus%20Structure))
  (bind (_age _expirationage _strength _stimuluslocation _receiverlocation _tag _bsuccessfullysensed) (Utilities|Struct|BreakAIStimulus Stimulus))
  (bind _returnvalue (Utilities|Name|MakeLiteralName "PlayerInVision"))
  (bind _blackboard (Variables|Default|GetBlackboard))
  (bind _returnvalue_2 (Class|AIPerceptionSystem|GetSenseClassforStimulus Stimulus))
  (if (== _returnvalue_2 "/Script/AIModule.AISense_Sight")
    (if _bsuccessfullysensed
      (AI|Components|Blackboard|SetValueasObject (Variables|Default|GetBlackboard) (Utilities|Name|MakeLiteralName "TargetActor") Actor)
      (AI|Components|Blackboard|SetValueasBool _blackboard _returnvalue true)
      (else
        (AI|Components|Blackboard|SetValueasBool _blackboard _returnvalue false)))
    (else
      (AI|Components|Blackboard|SetValueasVector (Variables|Default|GetBlackboard) (Utilities|Name|MakeLiteralName "TargetLocation") _stimuluslocation))))

(event EventBeginPlay
  (AI|RunBehaviorTree "/Game/MyContent/Blueprints/AI/BT_EnemyBehaviorTree.BT_EnemyBehaviorTree"))

(fn ConstructionScript)